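; Emissive item Blueprint that pairs its static mesh with a colored point light, which fades out when the item is hidden.
; The Construction Script sets the light from exposed color and intensity values and, when an emissive material is set, tints a dynamic instance of it to match.
; HideItem extends the parent event, keeps the light unhidden, then runs a rate-adjustable timeline that lerps its intensity to zero.
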(event Custom|TurnOffLight
  (Components|Timeline|SetPlayRate (Variables|Default|GetTurnOffLightAnimation) (Variables|Default|GetLightOffAnimationRade))
  (bind _alpha (Timeline|TurnOffLightAnimation PlayFromStart)
    (:Update
      (Rendering|Components|Light|SetIntensity (Variables|Default|GetPointLight) (Math|Float|Lerp (Variables|Default|GetLightIntensity) 0.0 _alpha)))))

(event EventBeginPlay
  (|CallParentFunction) ; This node is disabled and will not be called.\nDrag off pins to build functionality.
)

(event Collision|EventActorBeginOverlap
  (params (OtherActor :type Actor%20Object%20Reference))
  (|CallParentFunction OtherActor) ; This node is disabled and will not be called.\nDrag off pins to build functionality.
)

(event EventTick
  (params (DeltaSeconds :type Float%20%28single-precision%29))
  (|CallParentFunction DeltaSeconds) ; This node is disabled and will not be called.\nDrag off pins to build functionality.
)

(event EventHideItem
  (|CallParentFunction)
  (Development|SetHiddeninGame (Variables|Default|GetPointLight) false true)
  (CallFunction|TurnOffLight))

(fn ConstructionScript
  (Utilities|FlowControl|Sequence
    (:then_0
      (Rendering|SetVisibility (Variables|Default|GetPointLight) (Variables|Default|GetEmissiveMaterial?) true)
      (Rendering|Components|Light|SetLightColor (Variables|Default|GetPointLight) (Variables|Default|GetLinearColor) true)
      (Rendering|Components|Light|SetIntensity (Variables|Default|GetPointLight) (Variables|Default|GetLightIntensity)))
    (:then_1
      (if (Variables|Default|GetEmissiveMaterial?)
        (bind _returnvalue (Rendering|Material|CreateDynamicMaterialInstance (Variables|Default|GetStaticMesh) 0 (Variables|Default|GetEmissiveMaterial) "None" :!class /Script/Engine.PrimitiveComponent))
        (Rendering|Material|SetVectorParameterValue _returnvalue (Variables|Default|GetEmissiveParameter) (Variables|Default|GetLinearColor) :!class /Script/Engine.MaterialInstanceDynamic)))))