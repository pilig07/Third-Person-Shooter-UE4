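; Base hitscan weapon actor for player or AI characters, firing automatically at a set rate while ammo remains on the owning Character.
; A timer re-runs HandleFiring; each shot consumes ammo, line-traces from camera or AI view, applies damage and spawns muzzle, trail and impact effects.
; Aiming and crouching tighten random cone spread, but crouch and ammo-pickup bindings are unwired.
; StopFiring waits out the pending shot interval before clearing the fire flag.
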(event Custom|SetWeaponOwner
  (params (NewOwner :type BP%20Character%20Object%20Reference))
  (bind _output_get (Variables|Mios|Player|SetCharacter NewOwner))
  (CallFunction|BindCharacterEvent)
  (Utilities|FlowControl|Sequence
    (:then_0
      (Variables|Mios|Player|SetPlayerController (.AsPlayer%20Controller (Utilities|Casting|CastToPlayerController (Pawn|GetController _output_get)))))
    (:then_1
      (Variables|Mios|IA|SetAIController (.AsAIController (Utilities|Casting|CastToAIController (Pawn|GetController _output_get)))))))

(event Custom|BindCharacterEvent
  (bind _character (Variables|Mios|Player|GetCharacter))
  (Utilities|IsValid _character
    (:Is%20Valid
      (EventDispatchers|AssignOnStartAiming _character (delegate Custom|OnCharacterStartAiming))
      (EventDispatchers|AssignOnEndAiming _character (delegate Custom|OnCharacterEndAiming)))))

(event Custom|OnCharacterStartCrouching
  (Variables|Mios|Shoot|Direccion|SetIsCharacterCrouched true))

(event Custom|OnCharacterEndCrouching
  (Variables|Mios|Shoot|Direccion|SetIsCharacterCrouched false))

(event Custom|OnCharacterAddingAmmo
  (params (Type :type E_AmmoType%20Enum :default "NewEnumerator0") (Ammo :type Integer))
  (if (Utilities|Enum|Equal(Enum) Type (Variables|Default|GetAmmo%20Type))
    (Default|CallOnAmmoChange Ammo)))

(event Custom|StartFiring
  ;[1 1 1] Firing
  (if (not (Variables|Mios|privare|GetWanttoFire?))
    (Variables|Mios|privare|SetWanttoFire? true)
    (Mios|Fire|HandleFiring)))

(event Custom|StopFiring
  ;[1 1 1] Firing
  (Utilities|FlowControl|Delay (Utilities|Time|GetTimerRemainingTimebyHandle (Variables|Mios|privare|GetFiringTimerHandle)))
  (Variables|Mios|privare|SetWanttoFire? false))

(event Custom|SetEquiped
  (params (Equiped? :type Boolean))
  ;[1 1 1] Equiped
  (bind _output_get (Variables|Mios|privare|SetEquiped? Equiped?))
  (Rendering|SetVisibility (Variables|Default|GetMesh_Weapon) _output_get true)
  (if (not Equiped?)
    (CallFunction|StopFiring)))

(event Custom|OnCharacterStartAiming
  (Variables|Mios|Shoot|Direccion|SetIsIronsight true))

(event Custom|OnCharacterEndAiming
  (Variables|Mios|Shoot|Direccion|SetIsIronsight false))

(event EventBeginPlay
  (Mios|Muzzle|SetUpMuzzleEffect)
  (Variables|Mios|item|SetTimeBetweenShoots (/ 1.0 (/ (Variables|Mios|item|GetShootPerMinute) 6e+01))))

(event Collision|EventActorBeginOverlap
  (params (OtherActor :type Actor%20Object%20Reference))
  (|CallParentFunction OtherActor) ; This node is disabled and will not be called.\nDrag off pins to build functionality.
)

(event EventTick
  (params (DeltaSeconds :type Float%20%28single-precision%29))
  (|CallParentFunction DeltaSeconds) ; This node is disabled and will not be called.\nDrag off pins to build functionality.
)

(fn ConstructionScript
  (|CallParentFunction))

(fn CanFire?
  (bind _character (Variables|Mios|Player|GetCharacter))
  (Utilities|IsValid _character
    (:Is%20Valid
      (return (Default|HasAmmo? _character (Variables|Default|GetAmmo%20Type))))))

(fn SetUpMuzzleEffect
  (bind _returnvalue (Effects|SpawnEmitterAttached "/Game/Effects/ParticleSystems/Weapons/AssaultRifle/Muzzle/P_AssaultRifle_MF.P_AssaultRifle_MF" (Variables|Default|GetScene_FirePoint) "None" "0, 0, 0" "0, 0, 0" "1.000000,1.000000,1.000000" "KeepRelativeOffset" false))
  (bind _output_get (Variables|Components|SetMuzzleFlash _returnvalue))
  (Components|Activation|Deactivate _output_get))

(fn SpawnTrailEffect
  (params (Target :type Vector))
  (bind _returnvalue (Effects|SpawnEmitteratLocation "/Game/Effects/ParticleSystems/Weapons/AssaultRifle/Muzzle/P_AssaultRifle_Trail.P_AssaultRifle_Trail" (Transformation|GetWorldLocation (Variables|Default|GetScene_FirePoint))))
  (Transformation|SetRelativeScale3D _returnvalue "3.000000,3.000000,3.000000")
  (Effects|Components|ParticleSystem|SetVectorParameter _returnvalue "ShockBeamEnd" Target))

(fn StopMuzzleEffect
  (Components|Activation|Deactivate (Variables|Components|GetMuzzleFlash)))

(fn StartMuzzleEffect
  (Components|Activation|Activate (Variables|Components|GetMuzzleFlash) false))

(fn FireWeapont
  (CallFunction|ConsumeAmmo)
  (Default|CallOnShooting)
  (bind (_impactpoint _impactnormal _hitactor) (Mios|Fire|ShotTrace))
  (Mios|Muzzle|SpawnImpactEffect _impactpoint _impactnormal _hitactor)
  (Mios|Muzzle|SpawnTrailEffect _impactpoint)
  (Mios|Fire|DamageTarget _hitactor)
  (Mios|Muzzle|StartMuzzleEffect)
  (Utilities|Time|SetTimerbyFunctionName self "StopMuzzleEffect" (Variables|Mios|item|GetMuzzleEffectTime)))

(fn HandleFiring
  (if (and (Variables|Mios|privare|GetWanttoFire?) (Mios|Muzzle|CanFire?))
    (Mios|Fire|FireWeapont)
    (bind _returnvalue (Utilities|Time|SetTimerbyFunctionName self "HandleFiring" (Variables|Mios|item|GetTimeBetweenShoots)))
    (Variables|Mios|privare|SetFiringTimerHandle _returnvalue)))

(fn GetTraceParameter
  (bind _aicontroller (Variables|Mios|IA|GetAIController))
  (bind _playercontroller (Variables|Mios|Player|GetPlayerController))
  (bind (_outlocation _outrotation) (Actor|GetActorEyesViewPoint _aicontroller))
  (bind _playercameramanager (Variables|/Script/Engine.PlayerController|GetPlayerCameraManager _playercontroller))
  (bind (_outlocation_2 _outrotation_2) (Actor|GetActorEyesViewPoint _playercameramanager))
  (Utilities|IsValid (Variables|Mios|Player|GetPlayerController)
    (:Is%20Valid
      (return _outlocation_2 (Math|Vector|GetForwardVector _outrotation_2)))
    (:Is%20Not%20Valid
      (Utilities|IsValid (Variables|Mios|IA|GetAIController)
        (:Is%20Valid
          (return _outlocation (Math|Vector|GetForwardVector _outrotation)))
        (:Is%20Not%20Valid
          (return "0, 0, 0" "0, 0, 0"))))))

(fn GetShotDirection
  (params (AimDirection :type Vector))
  (return (Math|Random|RandomUnitVectorinConeinDegrees AimDirection (Math|Trig|DegreesToRadians (* (Variables|Mios|Shoot|Direccion|GetShootSpread) (- 1.0 (+ (select (Variables|Mios|Shoot|Direccion|GetIsCharacterCrouched) 0.25 0.0) (select (Variables|Mios|Shoot|Direccion|GetIsIronsight) 0.25 0.0))))))))

(fn ShotTrace
  (bind (_location _direction) (Mios|Fire|GetTraceParameter))
  (bind _outhit (Collision|LineTraceByChannel _location (+ _location (* (Mios|Fire|GetShotDirection _direction) (+ (Variables|Mios|Shoot|GetShotDistance) 1e+03))) "TraceTypeQuery3" false (Utilities|Array|MakeArray (Variables|Mios|Player|GetCharacter)) "None" true "(R=1.000000,G=0.000000,B=0.000000,A=1.000000)" "(R=0.000000,G=1.000000,B=0.000000,A=1.000000)" 1.0))
  (return (select (.bBlockingHit (Collision|BreakHitResult _outhit)) (.ImpactPoint (Collision|BreakHitResult _outhit)) (.TraceEnd (Collision|BreakHitResult _outhit))) (.ImpactNormal (Collision|BreakHitResult _outhit)) (.HitActor (Collision|BreakHitResult _outhit))))

(fn SpawnImpactEffect
  (params (ImpactPoint :type Vector) (ImpactNormal :type Vector) (Actor :type Actor%20Object%20Reference))
  (Utilities|IsValid Actor
    (:Is%20Valid
      (Effects|SpawnEmitteratLocation (select (Utilities|ClassIsChildOf (Utilities|GetClass Actor) "/Script/Engine.Pawn") "/Game/Effects/ParticleSystems/Gameplay/Player/P_body_bullet_impact.P_body_bullet_impact" "/Game/Effects/ParticleSystems/Weapons/AssaultRifle/Impacts/P_AssaultRifle_IH.P_AssaultRifle_IH") ImpactPoint (Math|Conversions|RotationFromXVector ImpactNormal)))))

(fn GetShootInstigator
  (bind _output_get (Variables|Default|SetController (Variables|Mios|Player|GetPlayerController)))
  (Utilities|IsValid _output_get
    (:Is%20Valid
      _)
    (:Is%20Not%20Valid
      (Variables|Default|SetController (Variables|Mios|IA|GetAIController))))
  (return (Variables|Default|GetController)))

(fn DamageTarget
  (params (Target :type Actor%20Object%20Reference))
  (Game|Damage|ApplyDamage Target (Variables|Default|GetShorDamage) (Mios|Fire|GetShootInstigator) (Variables|Mios|Player|GetCharacter)))

(fn ConsumeAmmo
  (bind _character (Variables|Mios|Player|GetCharacter))
  (Utilities|IsValid _character
    (:Is%20Valid
      (bind _ammo (Default|ConsumeAmmo _character (Variables|Default|GetAmmo%20Type)))
      (Default|CallOnAmmoChange _ammo))))

(fn GetAmmoCount
  (Utilities|IsValid (Variables|Mios|Player|GetCharacter)
    (:Is%20Valid
      (return (Default|GetAmmoCount (Variables|Mios|Player|GetCharacter) (Variables|Default|GetAmmo%20Type))))
    (:Is%20Not%20Valid
      (return 0))))