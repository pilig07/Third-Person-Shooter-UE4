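; AI controller for bot characters that runs the BT_Bot behavior tree and targets the player.
; On BeginPlay it applies the bot's settings, optionally disabling movement and copying LoseSight and any preset Target to the blackboard.
; AI perception updates set focus and the blackboard target on a detected player character.
; ShootEnemy toggles the pawn's firing and aiming by line of sight, returning whether it can shoot.
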(event OnPerceptionUpdated(AIPerception)
  (params (UpdatedActors :type Array%20of%20Actor%20Object%20References))
  (bind _array_element (Utilities|Array|ForEachLoopwithBreak UpdatedActors :!label _label)
    (:LoopBody
      (bind _asbp_tps_player_character (Utilities|Casting|CastToBP_TPS_PlayerCharacter _array_element))
      (CallFunction|AttackCharacter _asbp_tps_player_character)
      (goto _label Break))))

(event Custom|SetUpAI
  (bind _returnvalue (AI|GetBlackboard 0))
  (AI|RunBehaviorTree "/Game/Parcial/BP/Base/IA/BT_Bot.BT_Bot")
  (bind _asbp_bot_character (Utilities|Casting|CastToBP_Bot_Character (Pawn|GetControlledPawn)))
  (Utilities|FlowControl|Sequence
    (:then_0
      (if (not (Variables|/Game/Parcial/BP/Base/IA/BP_Bot_Character.BP_Bot_Character_C|GetCanWalk? _asbp_bot_character))
        (Pawn|Components|CharacterMovement|DisableMovement (Variables|/Script/Engine.Character|GetCharacterMovement _asbp_bot_character))))
    (:then_1
      (Utilities|IsValid _returnvalue
        (:Is%20Valid
          (AI|Components|Blackboard|SetValueasBool _returnvalue (Variables|Default|GetLoseSightKeyName) (Variables|/Game/Parcial/BP/Base/IA/BP_Bot_Character.BP_Bot_Character_C|GetLoseSight? _asbp_bot_character)))))
    (:then_2
      (Utilities|IsValid (Variables|/Game/Parcial/BP/Base/IA/BP_Bot_Character.BP_Bot_Character_C|GetTarget _asbp_bot_character)
        (:Is%20Valid
          (CallFunction|SetTarget (Variables|/Game/Parcial/BP/Base/IA/BP_Bot_Character.BP_Bot_Character_C|GetTarget _asbp_bot_character)))))))

(event Custom|SetTarget
  (params (ObjectValue :type Object%20Object%20Reference))
  ;[1 1 1] Setear valores de blackboard
  (AI|Components|Blackboard|SetValueasObject (AI|GetBlackboard 0) (Variables|Default|GetTargetKeyName) ObjectValue))

(event Custom|AttackCharacter
  (params (Character :type BP%20Character%20Object%20Reference))
  (AI|SetFocus Character)
  (CallFunction|SetTarget Character))

(event EventBeginPlay
  (CallFunction|SetUpAI))

(event EventTick
  (params (DeltaSeconds :type Float%20%28single-precision%29)))

(fn ConstructionScript)

(fn ShootEnemy
  (params (Enemy :type BP%20Character%20Object%20Reference))
  (bind _asbp_character (Utilities|Casting|CastToBP_Character (Pawn|GetControlledPawn)))
  (if (Controller|LineOfSightTo Enemy "0, 0, 0" false)
    (Default|StartFiringWeapon _asbp_character)
    (Default|StartAiming _asbp_character)
    (return true)
    (else
      (Default|StopFiringWeapon _asbp_character)
      (Default|StopAiming _asbp_character)
      (return false))))