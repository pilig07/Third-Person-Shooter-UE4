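; Base interactable actor that gates and runs an interaction requested with another actor.
; Interact checks CanInteract, which requires a valid actor and blocks repeats when InteractOnce is set and WasInteracted is true.
; It then runs Interaction, a default hook that simply returns true, stores the result in WasInteracted and calls the OnInteracted dispatcher on success.
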(event EventBeginPlay)

(event Collision|EventActorBeginOverlap
  (params (OtherActor :type Actor%20Object%20Reference)))

(event EventTick
  (params (DeltaSeconds :type Float%20%28single-precision%29)))

(fn ConstructionScript)

(fn Interaction
  (params (Actor :type Actor%20Object%20Reference))
  (return true))

(fn CanInteract?
  (params (Actor :type Actor%20Object%20Reference))
  (Utilities|IsValid Actor
    (:Is%20Valid
      (return (Math|Boolean|NANDBoolean (Variables|Default|GetWasInteracted) (Variables|Default|GetInteractOnce))))
    (:Is%20Not%20Valid
      (return false))))

(fn Interact
  (params (Actor :type Actor%20Object%20Reference))
  (bind _returnvalue (CallFunction|CanInteract? Actor))
  (if _returnvalue
    (bind _sucess (CallFunction|Interaction Actor))
    (bind _output_get (Variables|Default|SetWasInteracted _sucess))
    (if _output_get
      (Default|CallOnInteracted)
      (return true)
      (else
        (return false)))
    (else
      (return false))))