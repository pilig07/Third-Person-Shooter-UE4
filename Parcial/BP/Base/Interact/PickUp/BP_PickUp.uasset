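; BP_PickUp is an interactable pickup that gives an item of a configurable class to a BP_Character.
; The construction script sizes the pickup sphere and previews the item as a scaled, collision-free child actor.
; BeginPlay destroys pickups without a valid class and sets the spin rate on RotatingMovement.
; Only characters can interact, which passes the class to ReceiveItem, then plays the item's sound and hides it.
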(event EventBeginPlay
  (|CallParentFunction)
  (Utilities|FlowControl|Sequence
    (:then_0
      (if (not (Utilities|IsValidClass (Variables|MC|Item|GetItemClass)))
        (Actor|DestroyActor)))
    (:then_1
      (Variables|/Script/Engine.RotatingMovementComponent|SetRotationRate (Variables|Default|GetRotatingMovement) (Math|Rotator|MakeRotator 0.0 0.0 (Variables|MC|Item|GetRotationRate))))))

(event Collision|EventActorBeginOverlap
  (params (OtherActor :type Actor%20Object%20Reference))
  (|CallParentFunction OtherActor) ; This node is disabled and will not be called.\nDrag off pins to build functionality.
)

(event EventTick
  (params (DeltaSeconds :type Float%20%28single-precision%29))
  (|CallParentFunction DeltaSeconds) ; This node is disabled and will not be called.\nDrag off pins to build functionality.
)

(fn ConstructionScript
  (Utilities|FlowControl|Sequence
    (:then_0
      (Transformation|SetRelativeLocation (Variables|Default|GetSphere) (Math|Vector|MakeVector 0.0 0.0 (Variables|MC|Item|GetItemHeight)) false false)
      (Components|Sphere|SetSphereRadius (Variables|Default|GetSphere) (Variables|MC|Item|GetPickUpRadius) true))
    (:then_1
      (if (Utilities|IsValidClass (Variables|MC|Item|GetItemClass))
        (bind _returnvalue (AddComponent|AddChildActorComponent false (Math|Transform|MakeTransform (Math|Vector|MakeVector 0.0 0.0 (Variables|MC|Item|GetItemHeight)) "0, 0, 0" "1.500000,1.500000,1.500000")))
        (bind _output_get (Variables|MC|Item|SetPickableActor _returnvalue))
        (Utilities|IsValid _output_get
          (:Is%20Valid
            (ChildActorComponent|SetChildActorClass (Variables|MC|Item|GetPickableActor) (Variables|MC|Item|GetItemClass))
            (Utilities|IsValid (Variables|/Script/Engine.ChildActorComponent|GetChildActor (Variables|MC|Item|GetPickableActor))
              (:Is%20Valid
                (Collision|SetActorEnableCollision (Variables|/Script/Engine.ChildActorComponent|GetChildActor (Variables|MC|Item|GetPickableActor)) false)))))))))

(fn CanInteract?
  (params (Actor :type Actor%20Object%20Reference))
  (bind _asbp_character (Utilities|Casting|CastToBP_Character Actor)
    (:then
      (bind _returnvalue (|CallParentFunction _asbp_character))
      (return _returnvalue))
    (:CastFailed
      (return false))))

(fn Interaction
  (params (Actor :type Actor%20Object%20Reference))
  (bind _asbp_character (Utilities|Casting|CastToBP_Character Actor)
    (:then
      (Default|ReceiveItem _asbp_character (Variables|MC|Item|GetItemClass))
      (Actor|SetLifeSpan 0.0)
      (bind _asbp_item (Utilities|Casting|CastToBP_Item (Variables|/Script/Engine.ChildActorComponent|GetChildActor (Variables|MC|Item|GetPickableActor))))
      (Default|PlayItemSound _asbp_item)
      (Default|HideItem _asbp_item)
      (bind _sucess (|CallParentFunction 0))
      (return _sucess))
    (:CastFailed
      (return false))))