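; BP_Coleccionable is a collectible pickup actor for the third-person player character, BP_TPS_PlayerCharacter.
; On BeginPlay it calls PickUP on the player pawn, so each instance notifies the player when it enters play.
; When the player character overlaps it, it calls PickUpADD on that character and destroys itself, leaving any pickup bookkeeping to the player Blueprint.
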(event EventBeginPlay
  (Default|PickUP (.AsBP%20TPS%20Player%20Character (Utilities|Casting|CastToBP_TPS_PlayerCharacter (Game|Player|GetPlayerPawn 0)))))

(event Collision|EventActorBeginOverlap
  (params (OtherActor :type Actor%20Object%20Reference))
  (if (== OtherActor (Game|GetPlayerCharacter 0))
    (Default|PickUpADD (.AsBP%20TPS%20Player%20Character (Utilities|Casting|CastToBP_TPS_PlayerCharacter (Game|Player|GetPlayerPawn 0))))
    (Actor|DestroyActor)))

(event EventTick
  (params (DeltaSeconds :type Float%20%28single-precision%29)))

(fn ConstructionScript)